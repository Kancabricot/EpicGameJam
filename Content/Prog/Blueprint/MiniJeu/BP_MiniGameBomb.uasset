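; Bomb-sorting minigame where the player presses X for left bombs and B for right ones, built on a parent providing start, victory and defeat.
; A self-recursive delayed event spawns bombs into an array; input always judges the oldest.
; Correct presses replace it with a blue or red mesh on its side, counting toward victory.
; Wrong presses or bombs reaching DefeatTrigger cause defeat; Reset clears bombs and meshes after either outcome.
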(event `SpawnBomb`
  (bind _spawnbomblocation (`self.SpawnBombLocation`))
  (bind _returnvalue (`|SpawnActorFromClass` "/Game/Prog/Blueprint/MiniJeu/BP_Bomb.BP_Bomb_C" (`KismetMathLibrary.MakeTransform` (`SceneComponent.K2_GetComponentLocation` _spawnbomblocation) (`SceneComponent.K2_GetComponentRotation` _spawnbomblocation) (5.0 5.0 5.0)) "Undefined" "MultiplyWithRoot" null null))
  (`KismetArrayLibrary.Array_Add` (`self.BombArray`) _returnvalue)
  (`KismetSystemLibrary.Delay` (`KismetMathLibrary.RandomFloatInRange` 0.3 0.8))
  (if (`self.b_InGame`)
    (`self.SpawnBomb`)))

(event `EnhancedInput|/Game/ThirdPerson/Input/Actions/IA_PressB`
  (params (ActionValue :type Boolean) (ElapsedSeconds :type "Float (double-precision)") (TriggeredSeconds :type "Float (double-precision)") (InputAction :type "InputAction Object Reference" :default "/Game/ThirdPerson/Input/Actions/IA_PressB.IA_PressB"))
  (bind _output (`|GetArrayItem` (`self.BombArray`)))
  (:`Started`
    (if (`/Game/Prog/Blueprint/MiniJeu/BP_Bomb.b_IsLeft` _output)
      (`NiagaraFunctionLibrary.SpawnSystemAtLocation` "/Game/VFX/VFX/NS_Explosion.NS_Explosion" (`SceneComponent.K2_GetComponentLocation` (`/Game/Prog/Blueprint/MiniJeu/BP_Bomb.SMTemp` _output)))
      (`KismetSystemLibrary.Delay` 0.2)
      (`self.Defeat`)
      (`self.Reset`)
      (else
        (`self.DeleteBomb` _output)))))

(event `self.Start`
  (`parent.Start`)
  (`self.SpawnBomb`)
  (set `self.b_InGame` true))

(event `EnhancedInput|/Game/ThirdPerson/Input/Actions/IA_PressX`
  (params (ActionValue :type Boolean) (ElapsedSeconds :type "Float (double-precision)") (TriggeredSeconds :type "Float (double-precision)") (InputAction :type "InputAction Object Reference" :default "/Game/ThirdPerson/Input/Actions/IA_PressX.IA_PressX"))
  (bind _output (`|GetArrayItem` (`self.BombArray`)))
  (:`Started`
    (if (`/Game/Prog/Blueprint/MiniJeu/BP_Bomb.b_IsLeft` _output)
      (`self.DeleteBomb` _output)
      (else
        (`NiagaraFunctionLibrary.SpawnSystemAtLocation` "/Game/VFX/VFX/NS_Explosion.NS_Explosion" (`SceneComponent.K2_GetComponentLocation` (`/Game/Prog/Blueprint/MiniJeu/BP_Bomb.SMTemp` _output)))
        (`KismetSystemLibrary.Delay` 0.2)
        (`self.Defeat`)
        (`self.Reset`)))))

(event `self.DefeatTrigger.OnComponentBeginOverlap`
  (params (OverlappedComponent :type "PrimitiveComponent Object Reference") (OtherActor :type "Actor Object Reference") (OtherComp :type "PrimitiveComponent Object Reference") (OtherBodyIndex :type Integer) (bFromSweep :type Boolean) (SweepResult :type "HitResult Structure (by ref)"))
  (bind _asbp_bomb (cast `/Game/Prog/Blueprint/MiniJeu/BP_Bomb` OtherActor))
  (`self.K2_DestroyActor` _asbp_bomb)
  (`self.Defeat`)
  (set `self.b_InGame` false)
  (`self.Reset`))

(fn `CheckIsFinish`
  (if (>= (`self.NBBomb`) (`self.MaxBombToDestroy`))
    (`NiagaraFunctionLibrary.SpawnSystemAtLocation` "/Game/VFX/VFX/NS_StarSuccess.NS_StarSuccess" (`SceneComponent.K2_GetComponentLocation` (`self.VFX Location`)))
    (`self.Victory`)
    (`self.Reset`)))

(fn `DeleteBomb`
  (params (BombTarget :type "/Game/Prog/Blueprint/MiniJeu/BP_Bomb Object Reference"))
  (bind (_relativelocation_x _relativelocation_y _relativelocation_z) (`KismetMathLibrary.BreakVector` (`SceneComponent.RelativeLocation` (select `bool` (`/Game/Prog/Blueprint/MiniJeu/BP_Bomb.b_IsLeft` (`local.BombTarget`)) :`false` (`self.RightBombSpawn`) :`true` (`self.LeftBombSpawn`)))))
  (bind _returnvalue (`AddComponent|NODE_AddStaticMeshComponent-0` :`RelativeTransform` (`KismetMathLibrary.MakeTransform` (`KismetMathLibrary.MakeVector` (+ _relativelocation_x (`KismetMathLibrary.RandomFloatInRange` -30.0 30.0)) (+ _relativelocation_y (`KismetMathLibrary.RandomFloatInRange` -30.0 30.0)) _relativelocation_z) (struct) (0.4 0.4 0.4))))
  (`KismetArrayLibrary.Array_Add` (`self.BombCompToDelete`) _returnvalue)
  (`PrimitiveComponent.SetMaterial` _returnvalue 0 (select `bool` (`/Game/Prog/Blueprint/MiniJeu/BP_Bomb.b_IsLeft` (`local.BombTarget`)) :`false` "/Game/Art/Mat/M_Red.M_Red" :`true` "/Game/Art/Mat/M_Blue.M_Blue" :!type "MaterialInterface Object Reference"))
  (`KismetArrayLibrary.Array_RemoveItem` (`self.BombArray`) BombTarget)
  (`self.K2_DestroyActor` BombTarget)
  (`/Engine/EditorBlueprintResources/StandardMacros.IncrementInt` (`self.NBBomb`)
    (:`  `
      (`self.CheckIsFinish`))))

(fn `Reset`
  (for _array_element (`self.BombCompToDelete`)
    (`ActorComponent.K2_DestroyComponent` _array_element))
  (`KismetArrayLibrary.Array_Clear` (`self.BombCompToDelete`))
  (set `self.b_InGame` false)
  (set `self.NBBomb` 0)
  (for _array_element_2 (`self.BombArray`)
    (`/Engine/EditorBlueprintResources/StandardMacros.IsValid` _array_element_2
      (:`Is Valid`
        (`self.K2_DestroyActor` _array_element_2))))
  (`KismetArrayLibrary.Array_Clear` (`self.BombArray`)))

(fn `UserConstructionScript`
  (`parent.UserConstructionScript`))