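; Rotation puzzle minigame with four pieces in a 2x2 grid, won by turning every piece upright.
; Start calls the parent, then gives each piece a random quarter-turn offset.
; MoveEvent uses D-pad direction to pick an adjacent piece, raising it and lowering the previous one.
; IA_PressA rotates the selected piece 90 degrees, then calls Victory if all four world rotations are near zero.
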(event `EnhancedInput|/Game/ThirdPerson/Input/Actions/IA_PressA`
  (params (ActionValue :type Boolean) (ElapsedSeconds :type "Float (double-precision)") (TriggeredSeconds :type "Float (double-precision)") (InputAction :type "InputAction Object Reference" :default "/Game/ThirdPerson/Input/Actions/IA_PressA.IA_PressA"))
  (:`Started`
    (`self.Rotation` (`self.PieceTemp`))))

(event `self.MoveEvent`
  (set `self.LastPieceTEmp` (`self.PieceTemp`))
  (if (== (`self.TopRightTemp`) (`self.PieceTemp`))
    (switch `/Game/Prog/Enumerator/E_DPad` (`self.E_DPad`)
      (:`NewEnumerator2`
        (set `self.PieceTemp` (`self.TopLeftTemp`)))
      (:`NewEnumerator3`
        (set `self.PieceTemp` (`self.BottomRightTemp`))))
    (elif (== (`self.TopLeftTemp`) (`self.PieceTemp`))
      (switch `/Game/Prog/Enumerator/E_DPad` (`self.E_DPad`)
        (:`NewEnumerator1`
          (set `self.PieceTemp` (`self.TopRightTemp`)))
        (:`NewEnumerator3`
          (set `self.PieceTemp` (`self.BottomLeftTemp`))))
      (elif (== (`self.BottomLeftTemp`) (`self.PieceTemp`))
        (switch `/Game/Prog/Enumerator/E_DPad` (`self.E_DPad`)
          (:`NewEnumerator0`
            (set `self.PieceTemp` (`self.TopLeftTemp`)))
          (:`NewEnumerator1`
            (set `self.PieceTemp` (`self.BottomRightTemp`))))
        (else
          (switch `/Game/Prog/Enumerator/E_DPad` (`self.E_DPad`)
            (:`NewEnumerator0`
              (set `self.PieceTemp` (`self.TopRightTemp`)))
            (:`NewEnumerator2`
              (set `self.PieceTemp` (`self.BottomLeftTemp`))))))))
  (`self.ShowSelection`))

(event `self.ReceiveBeginPlay`
  (set `self.PieceTemp` (`self.TopLeftTemp`))
  (`self.ShowSelection`))

(event `self.Start`
  ;[1 1 1] Start
  (`parent.Start`)
  (`self.SetUpRotation` (`self.TopLeftTemp`))
  (`self.SetUpRotation` (`self.TopRightTemp`))
  (`self.SetUpRotation` (`self.BottomLeftTemp`))
  (`self.SetUpRotation` (`self.BottomRightTemp`)))

(fn `CheckAllRotation`
  (if (== (`SceneComponent.K2_GetComponentRotation` (`self.TopRightTemp`)) (struct) :`ErrorTolerance` 10.0)
    (if (== (`SceneComponent.K2_GetComponentRotation` (`self.TopLeftTemp`)) (struct) :`ErrorTolerance` 10.0)
      (if (== (`SceneComponent.K2_GetComponentRotation` (`self.BottomLeftTemp`)) (struct) :`ErrorTolerance` 10.0)
        (if (== (`SceneComponent.K2_GetComponentRotation` (`self.BottomRightTemp`)) (struct) :`ErrorTolerance` 10.0)
          (`self.Victory`))))))

(fn `Rotation`
  (params (TargetPiece :type "StaticMeshComponent Object Reference"))
  (`SceneComponent.K2_SetWorldRotation` TargetPiece (`KismetMathLibrary.ComposeRotators` (`SceneComponent.K2_GetComponentRotation` TargetPiece) (struct :`Yaw` 90.0)) false false)
  (`self.CheckAllRotation`))

(fn `SetUpRotation`
  (params (PieceTarget :type "SceneComponent Object Reference"))
  (`SceneComponent.K2_AddLocalRotation` PieceTarget (select `int` (`KismetMathLibrary.RandomIntegerInRange` 0 3) :`0` (struct) :`1` (struct :`Yaw` 90.0) :`2` (struct :`Yaw` 180.0) :`3` (struct :`Yaw` -90.0) :!type "Rotator Structure") false false))

(fn `ShowSelection`
  (bind _piecetemp (`self.PieceTemp`))
  (bind _lastpiecetemp (`self.LastPieceTEmp`))
  (`SceneComponent.K2_SetRelativeLocation` _piecetemp (+ (`SceneComponent.RelativeLocation` _piecetemp) (0.0 0.0 20.0)) false false)
  (`/Engine/EditorBlueprintResources/StandardMacros.IsValid` _lastpiecetemp
    (:`Is Valid`
      (`SceneComponent.K2_SetRelativeLocation` _lastpiecetemp (+ (`SceneComponent.RelativeLocation` _lastpiecetemp) (0.0 0.0 -20.0)) false false))))

(fn `UserConstructionScript`
  (`parent.UserConstructionScript`))