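; Manager Blueprint that randomly assigns an effect to each mini-game at the start of play.
; On BeginPlay it shuffles the MiniGame and EEffect arrays independently, then pairs them by index, setting each mini-game's EEffect to the matching entry.
; Each assigned effect name is printed to screen.
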(event `self.ReceiveBeginPlay`
  (`KismetArrayLibrary.Array_Shuffle` (`self.MiniGame`))
  (`KismetArrayLibrary.Array_Shuffle` (`self.E_Effect`))
  (for (_array_element _array_index) (`self.MiniGame`)
    (bind _output (`|GetArrayItem` (`self.E_Effect`) _array_index))
    (set `/Game/Prog/Blueprint/MiniJeu/BP_MiniJeuParent.E_Effect` _output _array_element)
    (`KismetSystemLibrary.PrintString` (`|GetEnumeratorNameAsString` _output))))

(fn `UserConstructionScript`)