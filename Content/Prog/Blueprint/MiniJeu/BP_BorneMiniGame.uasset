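; BP_BorneMiniGame is a mini-game terminal that the player can approach to start a mini-game.
; Entering its collision zone flags BP_Player as near, hands it a reference to the terminal, hides the input indication and switches the screen to a hologram material.
; Leaving clears the flag and reference and restores the screen material, but not the indication.
; StartMiniGame only flags the given player as in a mini-game.
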(event `self.Collision Zone.OnComponentBeginOverlap`
  (params (OverlappedComponent :type "PrimitiveComponent Object Reference") (OtherActor :type "Actor Object Reference") (OtherComp :type "PrimitiveComponent Object Reference") (OtherBodyIndex :type Integer) (bFromSweep :type Boolean) (SweepResult :type "HitResult Structure (by ref)"))
  (bind _asbp_player (cast `/Game/Prog/Blueprint/BP_Player` OtherActor))
  (set `/Game/Prog/Blueprint/BP_Player.b_NearToBorne` true _asbp_player)
  (set `/Game/Prog/Blueprint/BP_Player.Borne` self _asbp_player)
  (`SceneComponent.SetVisibility` (`self.ImputIndication`) false false)
  (`PrimitiveComponent.SetMaterial` (`self.SM_Borne_Minijeu_B`) 1 "/Game/Assets/BorneForMiniGame/MI_Hologram.MI_Hologram"))

(event `self.Collision Zone.OnComponentEndOverlap`
  (params (OverlappedComponent :type "PrimitiveComponent Object Reference") (OtherActor :type "Actor Object Reference") (OtherComp :type "PrimitiveComponent Object Reference") (OtherBodyIndex :type Integer))
  (bind _asbp_player (cast `/Game/Prog/Blueprint/BP_Player` OtherActor))
  (`PrimitiveComponent.SetMaterial` (`self.SM_Borne_Minijeu_B`) 1 "/Game/Assets/BorneForMiniGame/M_BorneEcran.M_BorneEcran")
  (set `/Game/Prog/Blueprint/BP_Player.Borne` null _asbp_player)
  (set `/Game/Prog/Blueprint/BP_Player.b_NearToBorne` false _asbp_player))

(fn `StartMiniGame`
  (params (PlayerTarget :type "/Game/Prog/Blueprint/BP_Player Object Reference"))
  (set `/Game/Prog/Blueprint/BP_Player.b_InMiniGame` true PlayerTarget))

(fn `UserConstructionScript`)