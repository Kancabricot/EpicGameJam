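; BP_MiniJeuSpammer is a timed button-mashing mini-game built on a parent class's Start.
; Each IA_PressA press fills a capped gauge, which drains a fixed amount per Tick, independent of delta time.
; While the game runs, Tick lerps the Jauge component's world scale to display the fill.
; After seven seconds, CheckEndGame calls Victory or Defeat against a 70% threshold, then resets the gauge.
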(event `EnhancedInput|/Game/ThirdPerson/Input/Actions/IA_PressA`
  (params (ActionValue :type Boolean) (ElapsedSeconds :type "Float (double-precision)") (TriggeredSeconds :type "Float (double-precision)") (InputAction :type "InputAction Object Reference" :default "/Game/ThirdPerson/Input/Actions/IA_PressA.IA_PressA"))
  ;[1 1 1] action du joueur en spamman la touche
  (:`Started`
    (set `self.JaugeSpammer` (+ (`self.JaugeSpammer`) 5.0))
    (if (>= (`self.JaugeSpammer`) 100.0)
      (set `self.JaugeSpammer` 100.0))))

(event `self.ReceiveTick`
  (params (DeltaSeconds :type "Float (single-precision)"))
  (bind _returnvalue (- (`self.JaugeSpammer`) 0.2))
  (bind _returnvalue_2 (/ (`self.JaugeSpammer`) 100.0))
  ;[1 1 1] diminution de la jauge a chaque Tick
  (if (`self.b_IsInGame`)
    (`SceneComponent.SetWorldScale3D` (`self.Jauge`) (`KismetMathLibrary.VLerp` (0.0 45.75 0.0) (160.0 45.75 0.0) _returnvalue_2))
    (`KismetSystemLibrary.PrintString` (`KismetStringLibrary.Conv_DoubleToString` _returnvalue_2) true true (struct :`G` 0.66 :`B` 1.0 :`A` 1.0) 0.0)
    (if (< _returnvalue 0.0)
      (set `self.JaugeSpammer` 0.0)
      (else
        (set `self.JaugeSpammer` _returnvalue)))))

(event `self.Start`
  ;[1 1 1] Start et Timer
  (`parent.Start`)
  (set `self.b_IsInGame` true)
  (`KismetSystemLibrary.K2_SetTimer` null "CheckEndGame" 7.0))

(fn `CheckEndGame`
  (if (>= (`self.JaugeSpammer`) 70.0)
    (`self.Victory`)
    (set `self.b_IsInGame` false)
    (else
      (`self.Defeat`)
      (set `self.b_IsInGame` false)))
  (`self.Reset`))

(fn `Reset`
  (set `self.JaugeSpammer` 0.0)
  (`SceneComponent.SetWorldScale3D` (`self.Jauge`) (0.0 45.75 0.0)))

(fn `UserConstructionScript`
  (`parent.UserConstructionScript`))