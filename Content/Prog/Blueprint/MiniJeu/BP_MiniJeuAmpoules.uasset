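; BP_MiniJeuAmpoules is a light-bulb reaction mini-game with four point lights mapped to the A, B, X and Y inputs.
; After a delayed start, a random light turns on and a timer gives the player a few seconds to press its button.
; Correct presses add to the score; wrong presses or timeouts cost a life, then another light is drawn.
; Reaching the target score calls Victory, losing all lives calls Defeat, and both reset the game.
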(event `EnhancedInput|/Game/ThirdPerson/Input/Actions/IA_PressB`
  (params (ActionValue :type Boolean) (ElapsedSeconds :type "Float (double-precision)") (TriggeredSeconds :type "Float (double-precision)") (InputAction :type "InputAction Object Reference" :default "/Game/ThirdPerson/Input/Actions/IA_PressB.IA_PressB"))
  ;[1 1 1] Vérif quand une touche est allumée
  (:`Started`
    (`self.CheckLight` (`self.PointLight_B`))))

(event `EnhancedInput|/Game/ThirdPerson/Input/Actions/IA_PressX`
  (params (ActionValue :type Boolean) (ElapsedSeconds :type "Float (double-precision)") (TriggeredSeconds :type "Float (double-precision)") (InputAction :type "InputAction Object Reference" :default "/Game/ThirdPerson/Input/Actions/IA_PressX.IA_PressX"))
  ;[1 1 1] Vérif quand une touche est allumée
  (:`Started`
    (`self.CheckLight` (`self.PointLight_X`))))

(event `EnhancedInput|/Game/ThirdPerson/Input/Actions/IA_PressA`
  (params (ActionValue :type Boolean) (ElapsedSeconds :type "Float (double-precision)") (TriggeredSeconds :type "Float (double-precision)") (InputAction :type "InputAction Object Reference" :default "/Game/ThirdPerson/Input/Actions/IA_PressA.IA_PressA"))
  ;[1 1 1] Vérif quand une touche est allumée
  (:`Started`
    (`self.CheckLight` (`self.PointLight_A`))))

(event `EnhancedInput|/Game/ThirdPerson/Input/Actions/IA_PressY`
  (params (ActionValue :type Boolean) (ElapsedSeconds :type "Float (double-precision)") (TriggeredSeconds :type "Float (double-precision)") (InputAction :type "InputAction Object Reference" :default "/Game/ThirdPerson/Input/Actions/IA_PressY.IA_PressY"))
  ;[1 1 1] Vérif quand une touche est allumée
  (:`Started`
    (`self.CheckLight` (`self.PointLight_Y`))))

(event `self.Start`
  ;[1 1 1] Light random s'allume quand le mini jeu est lancé
  (`parent.Start`)
  (`KismetSystemLibrary.K2_SetTimerDelegate` (delegate `LightOn`) 2.0))

(event `LightOn`
  ;[1 1 1] Light random s'allume quand le mini jeu est lancé
  (`self.SetLightsOn`))

(event `self.ReceiveBeginPlay`
  (bind _lights_array (`self.Lights_Array`))
  ;[1 1 1] Set de l'index des Lights
  (`KismetArrayLibrary.Array_Add` _lights_array (`self.PointLight_A`))
  (`KismetArrayLibrary.Array_Add` _lights_array (`self.PointLight_X`))
  (`KismetArrayLibrary.Array_Add` _lights_array (`self.PointLight_Y`))
  (`KismetArrayLibrary.Array_Add` _lights_array (`self.PointLight_B`)))

(fn `CheckLight`
  (params (Target :type "LightComponentBase Object Reference"))
  (if (> (`LightComponentBase.Intensity` Target) 0.0)
    (`KismetSystemLibrary.PrintString` "Success")
    (set `self.NBToWin` (+ 1 (`self.NBToWin`)))
    (`self.CheckWin`)
    (else
      (`KismetSystemLibrary.PrintString` "Hello")
      (set `self.Life` (- (`self.Life`) 1))
      (`self.CheckLose`))))

(fn `CheckLose`
  (if (<= (`self.Life`) 0)
    (`self.Defeat`)
    (`self.Reset`)
    (else
      (`self.SetLightOff`))))

(fn `CheckWin`
  (if (>= (`self.NBToWin`) (`self.NBForWin`))
    (`self.Victory`)
    (`self.Reset`)
    (else
      (`self.SetLightOff`))))

(fn `Reset`
  (set `self.NBToWin` 0)
  (set `self.Life` 2)
  (`LightComponent.SetIntensity` (`self.Lights_Array`) 0.0)
  (`KismetSystemLibrary.K2_ClearAndInvalidateTimerHandle` (`self.TimerRef`)))

(fn `SetLightOff`
  (`LightComponent.SetIntensity` (`self.Lights_Array`) 0.0)
  (`self.SetLightsOn`))

(fn `SetLightsOn`
  (`LightComponent.SetIntensity` (`KismetArrayLibrary.Array_Random` (`self.Lights_Array`)) 5000.0)
  (bind _returnvalue (`KismetSystemLibrary.K2_SetTimer` null "Timer" 3.0))
  (set `self.TimerRef` _returnvalue))

(fn `Timer`
  (set `self.Life` (- (`self.Life`) 1))
  (`self.CheckLose`))

(fn `UserConstructionScript`
  (`parent.UserConstructionScript`))