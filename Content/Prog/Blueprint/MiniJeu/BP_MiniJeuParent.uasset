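; Parent Blueprint for mini-games, providing input setup, a timed run and the hand-back to the player.
; Start adds the mini-game mapping context for the player, then calls Victory after a fixed delay, which clears the player's mini-game flag and blends the view back to them.
; Move input sets a D-pad direction enum; the face buttons only print debug text and the Move function's switch is empty.
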(event `EnhancedInput|/Game/ThirdPerson/Input/Actions/IA_Move`
  (params (ActionValue :type "Vector2D Structure") (ElapsedSeconds :type "Float (double-precision)") (TriggeredSeconds :type "Float (double-precision)") (InputAction :type "InputAction Object Reference" :default "/Game/ThirdPerson/Input/Actions/IA_Move.IA_Move"))
  (:`Started`
    (if (> ActionValue_X 5.0)
      (set `self.E_DPad` "NewEnumerator1")
      (elif (< ActionValue_X -5.0)
        (set `self.E_DPad` "NewEnumerator2")
        (elif (> ActionValue_Y 5.0)
          (set `self.E_DPad` "NewEnumerator0")
          (else
            (set `self.E_DPad` "NewEnumerator3")))))))

(event `EnhancedInput|/Game/ThirdPerson/Input/Actions/IA_PressA`
  (params (ActionValue :type Boolean) (ElapsedSeconds :type "Float (double-precision)") (TriggeredSeconds :type "Float (double-precision)") (InputAction :type "InputAction Object Reference" :default "/Game/ThirdPerson/Input/Actions/IA_PressA.IA_PressA"))
  (:`Started`
    (`KismetSystemLibrary.PrintString` "A")))

(event `EnhancedInput|/Game/ThirdPerson/Input/Actions/IA_PressB`
  (params (ActionValue :type Boolean) (ElapsedSeconds :type "Float (double-precision)") (TriggeredSeconds :type "Float (double-precision)") (InputAction :type "InputAction Object Reference" :default "/Game/ThirdPerson/Input/Actions/IA_PressB.IA_PressB"))
  (:`Started`
    (`KismetSystemLibrary.PrintString` "B")))

(event `EnhancedInput|/Game/ThirdPerson/Input/Actions/IA_PressX`
  (params (ActionValue :type Boolean) (ElapsedSeconds :type "Float (double-precision)") (TriggeredSeconds :type "Float (double-precision)") (InputAction :type "InputAction Object Reference" :default "/Game/ThirdPerson/Input/Actions/IA_PressX.IA_PressX"))
  (:`Started`
    (`KismetSystemLibrary.PrintString` "X")))

(event `EnhancedInput|/Game/ThirdPerson/Input/Actions/IA_PressY`
  (params (ActionValue :type Boolean) (ElapsedSeconds :type "Float (double-precision)") (TriggeredSeconds :type "Float (double-precision)") (InputAction :type "InputAction Object Reference" :default "/Game/ThirdPerson/Input/Actions/IA_PressY.IA_PressY"))
  (:`Started`
    (`KismetSystemLibrary.PrintString` "Y")))

(event `Start`
  (`self.SetInput`)
  (`KismetSystemLibrary.Delay` 20.0)
  (`self.Victory`))

(fn `Move`
  (switch `/Game/Prog/Enumerator/E_DPad` (`self.E_DPad`)))

(fn `SetInput`
  (bind _returnvalue (pcsubsystem `EnhancedInputLocalPlayerSubsystem` (`GameplayStatics.GetPlayerController` (`self.Player Index`))))
  (`KismetSystemLibrary.PrintString` "Start input")
  (`/Engine/EditorBlueprintResources/StandardMacros.IsValid` _returnvalue
    (:`Is Valid`
      (`KismetSystemLibrary.PrintString` "Switch input")
      (`EnhancedInputSubsystemInterface.AddMappingContext` _returnvalue "/Game/ThirdPerson/Input/IMC_MiniGame.IMC_MiniGame" 0 (struct))
      (`KismetSystemLibrary.PrintString` "End input"))))

(fn `UserConstructionScript`)

(fn `Victory`
  (bind _playerref (`self.PlayerRef`))
  (set `/Game/Prog/Blueprint/BP_Player.b_InMiniGame` false _playerref)
  (`PlayerController.SetViewTargetWithBlend` (`GameplayStatics.GetPlayerController` (`/Game/Prog/Blueprint/BP_Player.Player Index` _playerref)) _playerref 0.0 "VTBlend_Linear" 0.0 false))