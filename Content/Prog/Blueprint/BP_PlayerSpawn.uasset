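; BP_PlayerSpawn sets up two local players when play begins.
; It gathers every PlayerStart, creates players 0 and 1, then spawns a BP_Player at the first and second start found.
; Each pawn is possessed by its matching player controller, and the second receives PlayerIndex 1.
; Start assignment follows the order GetAllActorsOfClass returns, with no check that two starts exist.
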(event `self.ReceiveBeginPlay`
  (bind _outactors (`GameplayStatics.GetAllActorsOfClass` "/Script/Engine.PlayerStart"))
  (set `self.PlayerStartArray` _outactors)
  (`GameplayStatics.CreatePlayer` 0)
  (bind _returnvalue (`|SpawnActorFromClass` "/Game/Prog/Blueprint/BP_Player.BP_Player_C" (`self.GetTransform` (`|GetArrayItem` (`self.PlayerStartArray`))) "Undefined" "MultiplyWithRoot" null 0 null))
  (`Controller.Possess` (`GameplayStatics.GetPlayerController` 0) _returnvalue)
  (`GameplayStatics.CreatePlayer` 1)
  (bind _returnvalue_2 (`|SpawnActorFromClass` "/Game/Prog/Blueprint/BP_Player.BP_Player_C" (`self.GetTransform` (`|GetArrayItem` (`self.PlayerStartArray`) 1)) "Undefined" "MultiplyWithRoot" null 1 null))
  (`Controller.Possess` (`GameplayStatics.GetPlayerController` 1) _returnvalue_2))

(fn `UserConstructionScript`)